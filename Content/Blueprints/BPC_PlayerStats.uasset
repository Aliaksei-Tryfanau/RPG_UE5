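; Player stats component that tracks health and stamina for BP_ThirdPersonCharacter and mirrors them to its main HUD.
; BeginPlay caches the owning character, and InitializeStats fills the health bar, health text and stamina bar.
; Decrease functions return true once the stat is depleted, while increase functions cap the current value at its maximum.
; Changes update the HUD directly, except IncreaseMaxStamina, which leaves the stamina bar untouched.
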(event `self.ReceiveBeginPlay`
  (bind _asbp_third_person_character (cast `/Game/ThirdPerson/Blueprints/BP_ThirdPersonCharacter` (`self.GetOwner`)))
  (set `self.Owner` _asbp_third_person_character))

(event `InitializeStats`
  (bind _mainhud (`/Game/ThirdPerson/Blueprints/BP_ThirdPersonCharacter.MainHUD` (`self.Owner`)))
  (`ProgressBar.SetPercent` (`/Game/UI/WBP_MainHUD.HealthBar` _mainhud) (/ (`self.CurrentHealth`) (`self.MaxHealth`)))
  (`TextBlock.SetText` (`/Game/UI/WBP_MainHUD.HealthText` _mainhud) (`KismetTextLibrary.Conv_DoubleToText` (`self.CurrentHealth`) "HalfToEven"))
  (`ProgressBar.SetPercent` (`/Game/UI/WBP_MainHUD.StaminaBar` (`/Game/ThirdPerson/Blueprints/BP_ThirdPersonCharacter.MainHUD` (`self.Owner`))) (/ (`self.CurrentStamina`) (`self.MaxStamina`))))

(fn `Decrease Stamina`
  (params (StaminaToSubtract :type "Float (double-precision)"))
  (returns (Exhausted :type Boolean))
  (bind _currentstamina (`self.CurrentStamina`))
  (if (> _currentstamina 0.0)
    (set `self.CurrentStamina` (- _currentstamina StaminaToSubtract))
    (`ProgressBar.SetPercent` (`/Game/UI/WBP_MainHUD.StaminaBar` (`/Game/ThirdPerson/Blueprints/BP_ThirdPersonCharacter.MainHUD` (`self.Owner`))) (/ (`self.CurrentStamina`) (`self.MaxStamina`)))
    (if (<= (`self.CurrentStamina`) 0.0)
      _
      (else
        (return false))))
  (return true))

(fn `DecreaseHealth`
  (params (Damage :type "Float (double-precision)"))
  (returns (IsPlayerDead :type Boolean))
  (bind _mainhud (`/Game/ThirdPerson/Blueprints/BP_ThirdPersonCharacter.MainHUD` (`self.Owner`)))
  (if (> (`self.CurrentHealth`) 0.0)
    (bind _output_get (set `self.CurrentHealth` (- (`self.CurrentHealth`) Damage)))
    (`ProgressBar.SetPercent` (`/Game/UI/WBP_MainHUD.HealthBar` _mainhud) (/ _output_get (`self.MaxHealth`)))
    (`TextBlock.SetText` (`/Game/UI/WBP_MainHUD.HealthText` _mainhud) (`KismetTextLibrary.Conv_DoubleToText` (`self.CurrentHealth`) "HalfToEven"))
    (if (<= (`self.CurrentHealth`) 0.0)
      _
      (else
        (return false))))
  (return true))

(fn `IncreaseHealth`
  (params (HealthToAdd :type "Float (double-precision)"))
  (bind _mainhud (`/Game/ThirdPerson/Blueprints/BP_ThirdPersonCharacter.MainHUD` (`self.Owner`)))
  (set `self.CurrentHealth` (+ HealthToAdd (`self.CurrentHealth`)))
  (if (> (`self.CurrentHealth`) (`self.MaxHealth`))
    (bind _output_get (set `self.CurrentHealth` (`self.MaxHealth`))))
  (`ProgressBar.SetPercent` (`/Game/UI/WBP_MainHUD.HealthBar` _mainhud) (/ _output_get (`self.MaxHealth`)))
  (`TextBlock.SetText` (`/Game/UI/WBP_MainHUD.HealthText` _mainhud) (`KismetTextLibrary.Conv_DoubleToText` (`self.CurrentHealth`) "HalfToEven")))

(fn `IncreaseMaxHealth`
  (params (MaxHealthToAdd :type "Float (double-precision)"))
  (set `self.MaxHealth` (+ MaxHealthToAdd (`self.MaxHealth`)))
  (`ProgressBar.SetPercent` (`/Game/UI/WBP_MainHUD.HealthBar` (`/Game/ThirdPerson/Blueprints/BP_ThirdPersonCharacter.MainHUD` (`self.Owner`))) (/ (`self.CurrentHealth`) (`self.MaxHealth`))))

(fn `IncreaseMaxStamina`
  (params (StaminaToAdd :type "Float (double-precision)"))
  (set `self.MaxStamina` (+ StaminaToAdd (`self.MaxStamina`))))

(fn `IncreaseStamina`
  (params (StaminaToAdd :type "Float (double-precision)"))
  (set `self.CurrentStamina` (+ StaminaToAdd (`self.CurrentStamina`)))
  (if (> (`self.CurrentStamina`) (`self.MaxStamina`))
    (set `self.CurrentStamina` (`self.MaxStamina`)))
  (`ProgressBar.SetPercent` (`/Game/UI/WBP_MainHUD.StaminaBar` (`/Game/ThirdPerson/Blueprints/BP_ThirdPersonCharacter.MainHUD` (`self.Owner`))) (/ (`self.CurrentStamina`) (`self.MaxStamina`))))
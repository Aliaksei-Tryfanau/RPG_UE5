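; Attack component for BP_ThirdPersonCharacter that runs a four-step melee combo of sword swings and a kick.
; Attack input plays the montage for the current index or buffers a press, which SwordAttackCombo consumes to continue or reset the chain.
; A looping timer sphere-traces along the blade, with a cooldown between hits, while the kick uses a single sphere trace.
; Hits on "Damageable"-tagged actors apply damage, camera shake and sound.
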(event `self.ReceiveBeginPlay`
  (bind _asbp_third_person_character (cast `/Game/ThirdPerson/Blueprints/BP_ThirdPersonCharacter` (`self.GetOwner`)))
  (bind _output_get (set `self.Owner` _asbp_third_person_character))
  (set `self.CharacterMesh` (`Character.Mesh` _output_get)))

(event `EnhancedInput|/Game/ThirdPerson/Input/Actions/IA_Attack`
  (params (ActionValue :type Boolean) (ElapsedSeconds :type "Float (double-precision)") (TriggeredSeconds :type "Float (double-precision)") (InputAction :type "InputAction Object Reference" :default "/Game/ThirdPerson/Input/Actions/IA_Attack.IA_Attack"))
  ;[1 1 1] Combo system
  ;;[1 1 1] Attack input
  (:`Started`
    (if (`self.CanAttack`)
      (`self.SwordAttack`))))

(event `AttackOne`
  ;[1 1 1] Combo system
  ;;[1 1 1] Attack one
  (`/Engine/EditorBlueprintResources/StandardMacros.DoOnce` false :!label _label
    (:`Completed`
      (`KismetSystemLibrary.Delay` 0.1)
      (`|PlayMontage` (`self.CharacterMesh`) "/Game/Characters/RPG_Character/Animations/SwordAttacks/Attack1_Montage.Attack1_Montage"
        (:`then`
          (set `self.AttackIndex` 1)
          (goto _label :!via `Reset`))))))

(event `SwordAttack`
  ;[1 1 1] Combo system
  ;;[1 1 1] Sword attack
  (if (`self.IsAttacking`)
    (set `self.SaveAttack` true)
    (else
      (set `self.IsAttacking` true)
      (switch `int` (`self.AttackIndex`) :!label _label_2
        (:`0`
          (`self.AttackOne`))
        (:`1`
          (`self.AttackTwo`))
        (:`2`
          (`self.AttackThree`))
        (:`3`
          (`self.AttackFour`))))))

(event `AttackTwo`
  ;[1 1 1] Combo system
  ;;[1 1 1] Attack two
  (`/Engine/EditorBlueprintResources/StandardMacros.DoOnce` false :!label _label_3
    (:`Completed`
      (`KismetSystemLibrary.Delay` 0.1)
      (`|PlayMontage` (`self.CharacterMesh`) "/Game/Characters/RPG_Character/Animations/SwordAttacks/Attack2_Montage.Attack2_Montage"
        (:`then`
          (set `self.AttackIndex` 2)
          (goto _label_3 :!via `Reset`))))))

(event `SwordAttackCombo`
  ;[1 1 1] Combo system
  ;;[1 1 1] Combo continue
  (if (`self.SaveAttack`)
    (set `self.SaveAttack` false)
    (goto _label_2)
    (else
      (`self.StopCombo`))))

(event `AttackThree`
  ;[1 1 1] Combo system
  ;;[1 1 1] Attack three
  (`/Engine/EditorBlueprintResources/StandardMacros.DoOnce` false :!label _label_4
    (:`Completed`
      (`KismetSystemLibrary.Delay` 0.1)
      (`|PlayMontage` (`self.CharacterMesh`) "/Game/Characters/RPG_Character/Animations/SwordAttacks/Kick_Montage.Kick_Montage"
        (:`then`
          (set `self.AttackIndex` 3)
          (goto _label_4 :!via `Reset`))))))

(event `StopCombo`
  ;[1 1 1] Combo system
  ;;[1 1 1] Stop combo
  (set `self.IsAttacking` false)
  (set `self.AttackIndex` 0))

(event `AttackFour`
  ;[1 1 1] Combo system
  ;;[1 1 1] Attack four
  (`/Engine/EditorBlueprintResources/StandardMacros.DoOnce` false :!label _label_5
    (:`Completed`
      (`KismetSystemLibrary.Delay` 0.1)
      (`|PlayMontage` (`self.CharacterMesh`) "/Game/Characters/RPG_Character/Animations/SwordAttacks/Attack3_Montage.Attack3_Montage"
        (:`then`
          (set `self.AttackIndex` 4)
          (goto _label_5 :!via `Reset`))))))

(event `StartSwordTrace`
  ;[1 1 1] Sword trace
  (bind _returnvalue (`KismetSystemLibrary.K2_SetTimerDelegate` (delegate `SwordTraceLoop`) 0.01 true))
  (set `self.SwordTraceHandle` _returnvalue))

(event `SwordTraceLoop`
  (bind _owner (`self.Owner`))
  ;[1 1 1] Sword trace
  (bind (_outhit _returnvalue) (`KismetSystemLibrary.SphereTraceSingle` :`Start` (`SceneComponent.K2_GetComponentLocation` (`/Game/ThirdPerson/Blueprints/BP_ThirdPersonCharacter.SwordTopPoint` _owner)) :`End` (`SceneComponent.K2_GetComponentLocation` (`/Game/ThirdPerson/Blueprints/BP_ThirdPersonCharacter.SwordBottomPoint` _owner)) :`Radius` 12.0 :`TraceChannel` "TraceTypeQuery1" :`DrawDebugType` "ForDuration" :`DrawTime` 1.0))
  (if _returnvalue
    (bind (_bblockinghit _binitialoverlap _time _distance _location _impactpoint _normal _impactnormal _physmat _hitactor) (`GameplayStatics.BreakHitResult` _outhit))
    (if (`Actor.ActorHasTag` _hitactor "Damageable")
      (`/Engine/EditorBlueprintResources/StandardMacros.DoOnce` false :!label _label_6
        (:`Completed`
          (`GameplayStatics.ApplyDamage` _hitactor 10.0)
          (`GameplayStatics.PlayWorldCameraShake` "/Game/Blueprints/BP_SwordHitShake.BP_SwordHitShake_C" _location 0.0 2000.0)
          (`self.PlaySwordHitSound`)
          (`KismetSystemLibrary.Delay` 0.5)
          (goto _label_6 :!via `Reset`))))))

(event `StopSwordTrace`
  ;[1 1 1] Sword trace
  (`KismetSystemLibrary.K2_ClearAndInvalidateTimerHandle` (`self.SwordTraceHandle`)))

(event `SphereTrace`
  (bind _returnvalue (`SceneComponent.K2_GetComponentLocation` (`/Game/ThirdPerson/Blueprints/BP_ThirdPersonCharacter.SphereTrace` (`self.Owner`))))
  ;[1 1 1] Sphere trace for kick
  (bind (_outhit _returnvalue_2) (`KismetSystemLibrary.SphereTraceSingle` :`Start` _returnvalue :`End` _returnvalue :`Radius` 25.0 :`TraceChannel` "TraceTypeQuery1" :`DrawDebugType` "ForDuration" :`DrawTime` 1.0))
  (if _returnvalue_2
    (bind (_bblockinghit _binitialoverlap _time _distance _location _impactpoint _normal _impactnormal _physmat _hitactor) (`GameplayStatics.BreakHitResult` _outhit))
    (if (`Actor.ActorHasTag` _hitactor "Damageable")
      (`GameplayStatics.ApplyDamage` _hitactor 10.0)
      (`GameplayStatics.PlayWorldCameraShake` "/Game/Blueprints/BP_SwordHitShake.BP_SwordHitShake_C" _location 0.0 2000.0)
      (`self.PlaySwordHitSound`))))

(event `PlaySwordHitSound`
  (`GameplayStatics.PlaySoundAtLocation` "/Game/Audio/SwordHit/MS_SwordHit.MS_SwordHit" (`Actor.K2_GetActorLocation` (`self.GetOwner`)) (struct) 1.0 1.0 0.0 "/Game/Audio/SA_Character.SA_Character" null null null))